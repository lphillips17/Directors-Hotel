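; CameroidInput is a Horror Engine Blueprint that handles input for the cameroid photo camera.
; Use switches off player input and enables controller input through helper calls.
; Its turn and look-up axes rotate the player pawn's view at half the raw axis value, and the TakePhoto action calls TakePhoto on the player.
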(event EventUse
  (params (HorrorEvent :type Boolean))
  (CallFunction|PlayerInput false)
  (CallFunction|ControllerInput true))

(event Input|ActionEvents|InputAction[HE]TakePhoto
  (params (Key :type Key%20Structure :default "None"))
  (:Pressed
    (bind _asmaster (CallFunction|GetPlayer))
    (Default|TakePhoto _asmaster)))

(event Input|AxisEvents|InputAxis[HE]Turn
  (params (AxisValue :type Float%20%28single-precision%29))
  (Pawn|Input|AddControllerYawInput (Game|Player|GetPlayerPawn 0) (/ AxisValue 2.0)))

(event Input|AxisEvents|InputAxis[HE]LookUp
  (params (AxisValue :type Float%20%28single-precision%29))
  (Pawn|Input|AddControllerPitchInput (Game|Player|GetPlayerPawn 0) (/ AxisValue 2.0)))

(fn ConstructionScript)