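; BP_3DMenuWidgets is an in-world 3D menu actor that moves the player's view between linked menus.
; On BeginPlay it binds to the transition event of its MenuWidgetClass widget and disables its own collision.
; A transition picks the target from LinkedMenus by index, though only index 0 is validated.
; It then swaps collision to the target actor and eases the player's view target over to it with a camera blend.
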(event Custom|TransitionToWidget
  (params (NewMenu :type BP%203D%20Menu%20Widgets%20Object%20Reference))
  ;[1 1 1] Camera transition
  (Collision|SetActorEnableCollision false)
  (Collision|SetActorEnableCollision NewMenu true)
  (Game|Player|SetViewTargetwithBlend (Game|GetPlayerController 0) NewMenu 2.0 "VTBlend_EaseInOut" 2.0 false))

(event Custom|OnTransitionBetweenMenus
  (params (MenuIndex :type Integer))
  ;[1 1 1] Calling the menu interger to swap too
  (if (Utilities|Array|IsValidIndex (Variables|Default|GetLinkedMenus))
    (CallFunction|TransitiontoWidget (Utilities|Array|Get(acopy) (Variables|Default|GetLinkedMenus) MenuIndex))))

(event EventBeginPlay
  ;[1 1 1] Calling the menu interger to swap too
  (bind _asmenu_widget_class (Utilities|Casting|CastToMenuWidgetClass (UserInterface|GetUserWidgetObject (Variables|Default|GetWidget))))
  (EventDispatchers|BindEventtoTransitiontoLinkedWidget _asmenu_widget_class (delegate Custom|OnTransitionBetweenMenus))
  (Collision|SetActorEnableCollision false))

(fn ConstructionScript)