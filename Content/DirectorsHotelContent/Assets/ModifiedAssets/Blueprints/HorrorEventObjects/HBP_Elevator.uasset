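; Interactive hotel elevator built as a horror event object, with two sliding doors that open when the player uses either one.
; Use fires a different horror event depending on the HasFlashlight flag, set by AlternativeUse, then opens the doors in both cases.
; Separate open and close timelines move the doors, firing their own horror events and closing automatically after a delay, with IsOpen blocking re-triggering until closed.
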(event EventAlternativeUse
  (params (HorrorEvent :type Boolean))
  (Utilities|HMCheckInteraction)
  (Variables|Default|SethasFlashlight true))

(event EventUse
  (params (HorrorEvent :type Boolean))
  (Utilities|HMCheckInteraction)
  (bind _asmaster (CallFunction|GetPlayer))
  (if (or (== (Variables|/Game/HorrorEngine/HorrorEngine.HorrorEngine_C|GetHitComponent _asmaster) (Variables|Default|GetDoor1)) (== (Variables|/Game/HorrorEngine/HorrorEngine.HorrorEngine_C|GetHitComponent _asmaster) (Variables|Default|GetDoor2)))
    (if (not (Variables|Default|GetisOpen))
      (if (Variables|Default|GethasFlashlight)
        (CallFunction|HorrorEventCheck "NewEnumerator6")
        (CallFunction|Open/On false)
        (else
          (CallFunction|HorrorEventCheck "NewEnumerator5")
          (CallFunction|Open/On false))))))

(event EventOpen/On
  (params (HorrorEvent :type Boolean))
  (CallFunction|HorrorEventCheck "NewEnumerator3")
  (Variables|Default|SetisOpen true)
  (bind (_direction _moveleftdoor _moverightdoor) (Timeline|OpenElevator PlayFromStart)
    (:Update
      (Transformation|SetRelativeLocation (Variables|Default|GetDoor1) _moveleftdoor false false)
      (Transformation|SetRelativeLocation (Variables|Default|GetDoor2) _moverightdoor false false))
    (:Finished
      (Utilities|FlowControl|Delay 5.0)
      (CallFunction|Close/Off false))))

(event EventClose/Off
  (params (HorrorEvent :type Boolean))
  (CallFunction|HorrorEventCheck "NewEnumerator4")
  (bind (_direction _moveleftdoor _moverightdoor) (Timeline|CloseElevator PlayFromStart)
    (:Update
      (Transformation|SetRelativeLocation (Variables|Default|GetDoor1) _moveleftdoor false false)
      (Transformation|SetRelativeLocation (Variables|Default|GetDoor2) _moverightdoor false false))
    (:Finished
      (Variables|Default|SetisOpen false))))

(fn ConstructionScript
  (Utilities|HMDefaultConstructions (Variables|HorrorEvent|GetCreateNewHorrorEvent)))