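; A horror event trigger volume that fires when the player pawn stays inside its box, optionally unlocking an achievement.
; Overlap starts a timeline whose rate derives from a configurable duration, and leaving the box stops it.
; The timeline's Event Check track runs the horror event check and unlocks the named achievement through the achievement subsystem if enabled.
; Construction applies default horror event setup and sizes the box, offsetting it by its extent.
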(event OnComponentBeginOverlap(OverlapTrigger)
  (params (OverlappedComponent :type Primitive%20Component%20Object%20Reference) (OtherActor :type Actor%20Object%20Reference) (OtherComp :type Primitive%20Component%20Object%20Reference) (OtherBodyIndex :type Integer) (bFromSweep :type Boolean) (SweepResult :type Hit%20Result%20Structure%20%28by%20ref%29))
  ;[1 1 1] Overlap Settings
  (if (== OtherActor (Game|Player|GetPlayerPawn 0))
    (Timeline|TriggerTimeline PlayFromStart
      (:EventCheck
        (CallFunction|HorrorEventCheck "NewEnumerator43")
        (if (Variables|Achievements|GetunlockAchievement)
          (Class|AchievementSubSystem|Unlock (Subsystems|GetAchievementSubSystem) (Variables|Achievements|GetAchievement%20Name)))))))

(event OnComponentEndOverlap(OverlapTrigger)
  (params (OverlappedComponent :type Primitive%20Component%20Object%20Reference) (OtherActor :type Actor%20Object%20Reference) (OtherComp :type Primitive%20Component%20Object%20Reference) (OtherBodyIndex :type Integer))
  ;[1 1 1] Overlap Settings
  (if (== OtherActor (Game|Player|GetPlayerPawn 0))
    (Timeline|TriggerTimeline Stop
      (:EventCheck
        (CallFunction|HorrorEventCheck "NewEnumerator43")
        (if (Variables|Achievements|GetunlockAchievement)
          (Class|AchievementSubSystem|Unlock (Subsystems|GetAchievementSubSystem) (Variables|Achievements|GetAchievement%20Name)))))))

(fn ConstructionScript
  (Utilities|HMDefaultConstructions (Variables|HorrorEvents|GetCreateNewHorrorEvent))
  (Components|Box|SetBoxExtent (Variables|Default|GetOverlapTrigger) (Variables|CollisionSettings|GetTriggerBoxExtent) true)
  (Transformation|SetRelativeLocation (Variables|Default|GetOverlapTrigger) (Variables|CollisionSettings|GetTriggerBoxExtent) false false)
  (CallFunction|PlayRate (Variables|Default|GetTriggerTimeline) (Variables|HorrorEvents|GetOverlapDuration%20%28Sec%29)))