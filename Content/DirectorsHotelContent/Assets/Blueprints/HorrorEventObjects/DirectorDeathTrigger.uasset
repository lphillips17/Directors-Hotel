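; Horror event trigger volume that runs an event check after the player stays inside it for a set duration, apparently for the director's death.
; Overlap starts a timeline paced by OverlapDurationSec and leaving stops it; its Event Check picks one of two HorrorEventCheck states from the saved DirectorDoor flag.
; The construction script runs shared horror-event setup and sizes the box, offsetting it by its extent so it grows from a corner.
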(event OnComponentBeginOverlap(OverlapTrigger)
  (params (OverlappedComponent :type Primitive%20Component%20Object%20Reference) (OtherActor :type Actor%20Object%20Reference) (OtherComp :type Primitive%20Component%20Object%20Reference) (OtherBodyIndex :type Integer) (bFromSweep :type Boolean) (SweepResult :type Hit%20Result%20Structure%20%28by%20ref%29))
  ;[1 1 1] Overlap Settings
  (if (== OtherActor (Game|Player|GetPlayerPawn 0))
    (Timeline|TriggerTimeline PlayFromStart
      (:EventCheck
        (bind _asmaster (CallFunction|GetPlayer))
        (if (Variables|/Game/HorrorEngine/Blueprints/Core/HE_GameInstance.HE_GameInstance_C|GetDirectorDoor (Variables|/Game/HorrorEngine/Blueprints/Core/HE_SaveGameComponent.HE_SaveGameComponent_C|GetGameInstance (Variables|/Game/HorrorEngine/HorrorEngine.HorrorEngine_C|GetHE_SaveGameComponent _asmaster)))
          (CallFunction|HorrorEventCheck "NewEnumerator3")
          (else
            (CallFunction|HorrorEventCheck "NewEnumerator4")))))))

(event OnComponentEndOverlap(OverlapTrigger)
  (params (OverlappedComponent :type Primitive%20Component%20Object%20Reference) (OtherActor :type Actor%20Object%20Reference) (OtherComp :type Primitive%20Component%20Object%20Reference) (OtherBodyIndex :type Integer))
  ;[1 1 1] Overlap Settings
  (if (== OtherActor (Game|Player|GetPlayerPawn 0))
    (Timeline|TriggerTimeline Stop
      (:EventCheck
        (bind _asmaster (CallFunction|GetPlayer))
        (if (Variables|/Game/HorrorEngine/Blueprints/Core/HE_GameInstance.HE_GameInstance_C|GetDirectorDoor (Variables|/Game/HorrorEngine/Blueprints/Core/HE_SaveGameComponent.HE_SaveGameComponent_C|GetGameInstance (Variables|/Game/HorrorEngine/HorrorEngine.HorrorEngine_C|GetHE_SaveGameComponent _asmaster)))
          (CallFunction|HorrorEventCheck "NewEnumerator3")
          (else
            (CallFunction|HorrorEventCheck "NewEnumerator4")))))))

(fn ConstructionScript
  (Utilities|HMDefaultConstructions (Variables|HorrorEvents|GetCreateNewHorrorEvent))
  (Components|Box|SetBoxExtent (Variables|Default|GetOverlapTrigger) (Variables|CollisionSettings|GetTriggerBoxExtent) true)
  (Transformation|SetRelativeLocation (Variables|Default|GetOverlapTrigger) (Variables|CollisionSettings|GetTriggerBoxExtent) false false)
  (CallFunction|PlayRate (Variables|Default|GetTriggerTimeline) (Variables|HorrorEvents|GetOverlapDuration%20%28Sec%29)))