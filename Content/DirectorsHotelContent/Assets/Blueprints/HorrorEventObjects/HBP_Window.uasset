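; Interactable window object that can trigger a horror event when the player uses it.
; Use runs the interaction check, then calls HorrorEventCheck with a fixed event type if the player's hit component is one of the four window meshes.
; The construction script runs the shared default setup, passing in CreateNewHorrorEvent.
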(event EventUse
  (params (HorrorEvent :type Boolean))
  (Utilities|HMCheckInteraction)
  (bind _asmaster (CallFunction|GetPlayer))
  (if (Math|Boolean|ORBoolean (== (Variables|/Game/HorrorEngine/HorrorEngine.HorrorEngine_C|GetHitComponent _asmaster) (Variables|Default|GetSM_Window_01)) (== (Variables|/Game/HorrorEngine/HorrorEngine.HorrorEngine_C|GetHitComponent _asmaster) (Variables|Default|GetSM_Window_02)) (== (Variables|/Game/HorrorEngine/HorrorEngine.HorrorEngine_C|GetHitComponent _asmaster) (Variables|Default|GetSM_Window_03)) (== (Variables|/Game/HorrorEngine/HorrorEngine.HorrorEngine_C|GetHitComponent _asmaster) (Variables|Default|GetSM_Window_04)))
    (CallFunction|HorrorEventCheck "NewEnumerator0")))

(fn ConstructionScript
  (Utilities|HMDefaultConstructions (Variables|HorrorEvent|GetCreateNewHorrorEvent)))