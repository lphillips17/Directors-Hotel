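; HBP_ElevatorButton is an interactable elevator button that fires horror events when used.
; On BeginPlay, a current-floor button loses collision and shows its lit material.
; When the player's hit component is the button, it runs a horror event check.
; With multiple triggers, flashlight possession selects the check's enum value; otherwise it uses a fixed value and calls CloseOff(false) on the elevator.
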(event EventUse
  (params (HorrorEvent :type Boolean))
  (Utilities|HMCheckInteraction)
  (bind _asmaster (CallFunction|GetPlayer))
  (if (== (Variables|/Game/HorrorEngine/HorrorEngine.HorrorEngine_C|GetHitComponent _asmaster) (Variables|Default|GetLiftButton))
    (if (Variables|Elevator|GetmultipleTriggers)
      (bind _asmaster_2 (CallFunction|GetPlayer))
      (if (Variables|/Game/HorrorEngine/HorrorEngine.HorrorEngine_C|GetHasFlashlight _asmaster_2)
        (CallFunction|HorrorEventCheck "NewEnumerator0")
        (else
          (CallFunction|HorrorEventCheck "NewEnumerator5")))
      (else
        (CallFunction|HorrorEventCheck "NewEnumerator0")
        (bind _returnvalue (Actor|GetActorOfClass "/Game/DirectorsHotelContent/Assets/Blueprints/HorrorEventObjects/HBP_Elevator.HBP_Elevator_C"))
        (Default|Close/Off _returnvalue false)))))

(event EventBeginPlay
  (if (Variables|Elevator|GetisCurrentFloor)
    (Collision|SetCollisionEnabled (Variables|Default|GetLiftButton) "NoCollision")
    (Rendering|Material|SetMaterial (Variables|Default|GetLiftButton) 0 "/Game/DirectorsHotelContent/Assets/Materials/ElevatorButton_On.ElevatorButton_On")))

(fn ConstructionScript
  (Utilities|HMDefaultConstructions (Variables|HorrorEvent|GetCreateNewHorrorEvent)))