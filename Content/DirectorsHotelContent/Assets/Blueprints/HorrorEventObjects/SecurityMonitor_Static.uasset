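; Horror event security monitor prop that toggles its screen between a fixed camera texture and black when used.
; The construction script applies the mesh and materials and creates a dynamic screen material, whose texture RefreshScreen sets from the OnOff state.
; Open/On and Close/Off refresh the screen and report the new state through HorrorEventCheck.
; Save hooks add to the player's asset cache and restore OnOff from a saved boolean slot.
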(event EventUse
  (params (HorrorEvent :type Boolean))
  ;[1 1 1] Interaction Settings
  (Utilities|HMCheckInteraction)
  (if (Variables|SecurityMonitorSettings|GetOn%20/%20Off)
    (CallFunction|Close/Off false)
    (else
      (CallFunction|Open/On false))))

(event EventBeginPlay
  ;[1 1 1] Event Begin Play
  (CallFunction|RefreshScreen))

(event EventRestoreSaveData
  (params (AssetSave :type Assets%20Save%20Structure))
  ;[0 1 0.5572] Save Settings
  (|BreakAssetSave AssetSave)
  (CallFunction|RefreshScreen))

(event EventCollectSaveData
  ;[0 1 0.5572] Save Settings
  (bind _asmaster (CallFunction|GetPlayer))
  (Utilities|Array|Add (Variables|/Game/HorrorEngine/Blueprints/Core/HE_SaveGameComponent.HE_SaveGameComponent_C|GetAssetCache (Variables|/Game/HorrorEngine/HorrorEngine.HorrorEngine_C|GetHE_SaveGameComponent _asmaster)) (|MakeAssetSave)))

(event EventOpen/On
  (params (HorrorEvent :type Boolean))
  ;[1 1 1] On / Off Settings
  (Utilities|HMCheckInteraction)
  (Variables|SecurityMonitorSettings|SetOn%20/%20Off true)
  (CallFunction|RefreshScreen)
  (CallFunction|HorrorEventCheck (select (Variables|SecurityMonitorSettings|GetOn%20/%20Off) "NewEnumerator4" "NewEnumerator3")))

(event EventClose/Off
  (params (HorrorEvent :type Boolean))
  ;[1 1 1] On / Off Settings
  (Utilities|HMCheckInteraction)
  (Variables|SecurityMonitorSettings|SetOn%20/%20Off false)
  (CallFunction|RefreshScreen)
  (CallFunction|HorrorEventCheck (select (Variables|SecurityMonitorSettings|GetOn%20/%20Off) "NewEnumerator4" "NewEnumerator3")))

(fn ConstructionScript
  (Utilities|HMDefaultConstructions (Variables|HorrorEvents|GetCreateNewHorrorEvent))
  (Components|StaticMesh|SetStaticMesh (Variables|Default|GetMonitor) (Variables|MeshSettings|GetMonitorMesh))
  (Rendering|Material|SetMaterial (Variables|Default|GetMonitor) 0 (Variables|MeshSettings|GetMonitorMaterial))
  (bind _returnvalue (Rendering|Material|CreateDynamicMaterialInstance (Variables|Default|GetMonitor) 1 (Variables|MeshSettings|GetScreenMaterial) "None" :!class /Script/Engine.PrimitiveComponent))
  (Variables|Default|SetScreenMaterialRef _returnvalue)
  (CallFunction|RefreshScreen))

(fn RefreshScreen
  (if (Variables|SecurityMonitorSettings|GetOn%20/%20Off)
    (Rendering|Material|SetTextureParameterValue (Variables|Default|GetScreenMaterialRef) "Texture" (select (Variables|SecurityMonitorSettings|GetOn%20/%20Off) (Variables|SecurityMonitorSettings|GetCameraTexture) "/Game/HorrorEngine/Textures/Empty_Black.Empty_Black"))
    (Rendering|Material|SetMaterial (Variables|Default|GetMonitor) 1 (select (Variables|SecurityMonitorSettings|GetOn%20/%20Off) (Variables|Default|GetScreenMaterialRef) "/Game/HorrorEngine/Materials/He_Noise.He_Noise"))
    (else
      (Rendering|Material|SetTextureParameterValue (Variables|Default|GetScreenMaterialRef) "Texture" "/Game/HorrorEngine/Textures/Empty_Black.Empty_Black")
      (Rendering|Material|SetMaterial (Variables|Default|GetMonitor) 1 (Variables|Default|GetScreenMaterialRef)))))