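; Horror event elevator with two sliding doors that the player can use to open.
; Timelines slide the doors, which close automatically after a pause, with state flags blocking overlapping moves.
; Tick latches whether the player has a flashlight; using a door opens it either way but triggers a different horror event for each case.
; Opening and closing fire their own events, and doors become interactable after a startup delay via a collision channel swap.
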(event EventBeginPlay
  (Collision|SetCollisionObjectType (Variables|Default|GetDoor1) "ECC_WorldStatic")
  (Utilities|FlowControl|Delay (Variables|Elevator|GetUsableDelay))
  (Collision|SetCollisionObjectType (Variables|Default|GetDoor1) "ECC_GameTraceChannel1"))

(event EventTick
  (params (DeltaSeconds :type Float%20%28single-precision%29))
  (if (not (Variables|Elevator|GethasFlashlight))
    (bind _asmaster (CallFunction|GetPlayer))
    (if (Variables|/Game/HorrorEngine/HorrorEngine.HorrorEngine_C|GetHasFlashlight _asmaster)
      (Variables|Elevator|SethasFlashlight true))))

(event EventUse
  (params (HorrorEvent :type Boolean))
  (Utilities|HMCheckInteraction)
  (bind _asmaster (CallFunction|GetPlayer))
  (if (or (== (Variables|/Game/HorrorEngine/HorrorEngine.HorrorEngine_C|GetHitComponent _asmaster) (Variables|Default|GetDoor1)) (== (Variables|/Game/HorrorEngine/HorrorEngine.HorrorEngine_C|GetHitComponent _asmaster) (Variables|Default|GetDoor2)))
    (if (Variables|Elevator|GethasFlashlight)
      (CallFunction|HorrorEventCheck "NewEnumerator6")
      (CallFunction|Open/On false)
      (else
        (CallFunction|HorrorEventCheck "NewEnumerator5")
        (CallFunction|Open/On false)))))

(event EventOpen/On
  (params (HorrorEvent :type Boolean))
  (if (not (Variables|Elevator|GetdoorsMoving))
    (if (not (Variables|Elevator|GetisOpen))
      (CallFunction|HorrorEventCheck "NewEnumerator3")
      (Variables|Elevator|SetdoorsMoving true)
      (bind (_direction _moveleftdoor _moverightdoor) (Timeline|OpenElevator PlayFromStart)
        (:Update
          (Transformation|SetRelativeLocation (Variables|Default|GetDoor1) _moveleftdoor false false)
          (Transformation|SetRelativeLocation (Variables|Default|GetDoor2) _moverightdoor false false))
        (:Finished
          (Variables|Elevator|SetdoorsMoving false)
          (Variables|Elevator|SetisOpen true)
          (Utilities|FlowControl|Delay 5.0)
          (CallFunction|Close/Off false))))))

(event EventClose/Off
  (params (HorrorEvent :type Boolean))
  (if (not (Variables|Elevator|GetdoorsMoving))
    (if (Variables|Elevator|GetisOpen)
      (CallFunction|HorrorEventCheck "NewEnumerator4")
      (Variables|Elevator|SetdoorsMoving true)
      (bind (_direction _moveleftdoor _moverightdoor) (Timeline|CloseElevator PlayFromStart)
        (:Update
          (Transformation|SetRelativeLocation (Variables|Default|GetDoor1) _moveleftdoor false false)
          (Transformation|SetRelativeLocation (Variables|Default|GetDoor2) _moverightdoor false false))
        (:Finished
          (Variables|Elevator|SetdoorsMoving false)
          (Variables|Elevator|SetisOpen false))))))

(fn ConstructionScript
  (Utilities|HMDefaultConstructions (Variables|HorrorEvent|GetCreateNewHorrorEvent)))