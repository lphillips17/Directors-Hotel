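; Painting actor that endlessly flickers or animates by swapping the material on its Painting component.
; From BeginPlay it loops through three HE_Painting materials in a back-and-forth order (1, 2, 3, 2), creating a new dynamic material instance at each swap.
; A custom event rolls random sub-second delays between swaps, though the loop back skips the roll, so the first frame reuses the previous delay.
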(event Custom|RandomFloat
  (Variables|Default|SetRandomValue (Math|Float|Clamp(Float) (Math|Random|RandomFloat) 0.0 1.0)))

(event EventBeginPlay
  (bind _randomvalue (Variables|Default|GetRandomValue))
  (CallFunction|RandomFloat)
  (Rendering|Material|CreateDynamicMaterialInstance (Variables|Default|GetPainting) 0 "/Game/HorrorEngine/Materials/MaterialInstances/HE_Painting.HE_Painting" "None" :!class /Script/Engine.PrimitiveComponent :!label _label)
  (Utilities|FlowControl|Delay _randomvalue)
  (CallFunction|RandomFloat)
  (Rendering|Material|CreateDynamicMaterialInstance (Variables|Default|GetPainting) 0 "/Game/HorrorEngine/Materials/MaterialInstances/HE_Painting2.HE_Painting2" "None" :!class /Script/Engine.PrimitiveComponent)
  (Utilities|FlowControl|Delay _randomvalue)
  (CallFunction|RandomFloat)
  (Rendering|Material|CreateDynamicMaterialInstance (Variables|Default|GetPainting) 0 "/Game/HorrorEngine/Materials/MaterialInstances/HE_Painting3.HE_Painting3" "None" :!class /Script/Engine.PrimitiveComponent)
  (Utilities|FlowControl|Delay _randomvalue)
  (CallFunction|RandomFloat)
  (Rendering|Material|CreateDynamicMaterialInstance (Variables|Default|GetPainting) 0 "/Game/HorrorEngine/Materials/MaterialInstances/HE_Painting2.HE_Painting2" "None" :!class /Script/Engine.PrimitiveComponent)
  (Utilities|FlowControl|Delay _randomvalue)
  (goto _label))

(fn ConstructionScript)