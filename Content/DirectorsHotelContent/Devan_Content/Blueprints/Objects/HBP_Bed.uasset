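; Interactive bed object for a horror game, reacting when the player uses it.
; On use it runs the shared interaction check, then fires a horror event check if the player's hit component is the bed mesh.
; Construction applies the shared default setup with a new horror event.
; An unconnected chain would unlock an achievement, fade in a widget and return to the main menu.
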(event EventUse
  (params (HorrorEvent :type Boolean))
  (Utilities|HMCheckInteraction)
  (bind _asmaster (CallFunction|GetPlayer))
  (if (== (Variables|/Game/HorrorEngine/HorrorEngine.HorrorEngine_C|GetHitComponent _asmaster) (Variables|Default|GetSM_Bed_01))
    (CallFunction|HorrorEventCheck "NewEnumerator0")))

(fn ConstructionScript
  (Utilities|HMDefaultConstructions (Variables|HorrorEvent|GetCreateNewHorrorEvent)))