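; HBP_ElevatorButton is an interactable elevator button in the horror event object set.
; When it represents the current floor, it starts with collision disabled on the button mesh and a lit "on" material.
; On use, it runs the shared interaction check and, if the player's hit component is the button, triggers a horror event check.
; Its construction script applies the default horror-object setup.
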(event EventUse
  (params (HorrorEvent :type Boolean))
  (Utilities|HMCheckInteraction)
  (bind _asmaster (CallFunction|GetPlayer))
  (if (== (Variables|/Game/HorrorEngine/HorrorEngine.HorrorEngine_C|GetHitComponent _asmaster) (Variables|Default|GetLiftButton))
    (CallFunction|HorrorEventCheck "NewEnumerator0")))

(event EventBeginPlay
  (if (Variables|Elevator|GetisCurrentFloor)
    (Collision|SetCollisionEnabled (Variables|Default|GetLiftButton) "NoCollision")
    (Rendering|Material|SetMaterial (Variables|Default|GetLiftButton) 0 "/Game/DirectorsHotelContent/Devan_Content/Materials/ElevatorButton_On.ElevatorButton_On")))

(fn ConstructionScript
  (Utilities|HMDefaultConstructions (Variables|HorrorEvent|GetCreateNewHorrorEvent)))